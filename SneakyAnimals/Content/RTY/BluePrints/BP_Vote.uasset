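; BP_Vote is a voting display actor with four lamps, lighting the option selected by VotedNum.
; BeginPlay creates dynamic lamp materials for the four components, stores them and four spotlights in parallel arrays, and switches all off.
; Hoverd, Clicked, Unhovered and Reset toggle the indexed lamp's LightPanner parameter and spotlight intensity together.
; Clicked also sets IsClicked; nothing here sets VotedNum or reads that flag.
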(event `self.ReceiveTick`
  (params (DeltaSeconds :type "Float (single-precision)")))

(event `self.ReceiveBeginPlay`
  (bind _arr_light (`self.arr_Light`))
  (bind _arr_spotlight (`self.arr_SpotLight`))
  (bind _returnvalue (`PrimitiveComponent.CreateDynamicMaterialInstance` (`self.1`) 3 "/Game/RTY/Materials/M_Lamp1_Inst.M_Lamp1_Inst" "None"))
  (bind _output_get (set `self.Light_1` _returnvalue))
  (`KismetArrayLibrary.Array_Add` (`self.arr_Light`) _output_get)
  (bind _returnvalue_2 (`PrimitiveComponent.CreateDynamicMaterialInstance` (`self.2`) 3 "/Game/RTY/Materials/M_Lamp1_Inst.M_Lamp1_Inst" "None"))
  (bind _output_get_2 (set `self.Light_2` _returnvalue_2))
  (`KismetArrayLibrary.Array_Add` (`self.arr_Light`) _output_get_2)
  (bind _returnvalue_3 (`PrimitiveComponent.CreateDynamicMaterialInstance` (`self.3`) 3 "/Game/RTY/Materials/M_Lamp1_Inst.M_Lamp1_Inst" "None"))
  (bind _output_get_3 (set `self.Light_3` _returnvalue_3))
  (`KismetArrayLibrary.Array_Add` (`self.arr_Light`) _output_get_3)
  (bind _returnvalue_4 (`PrimitiveComponent.CreateDynamicMaterialInstance` (`self.4`) 3 "/Game/RTY/Materials/M_Lamp1_Inst.M_Lamp1_Inst" "None"))
  (bind _output_get_4 (set `self.Light_4` _returnvalue_4))
  (`KismetArrayLibrary.Array_Add` _arr_light _output_get_4)
  (for _array_element _arr_light
    (`MaterialInstanceDynamic.SetScalarParameterValue` _array_element "LightPanner" 0.0))
  (`KismetArrayLibrary.Array_Add` _arr_spotlight (`self.SpotLight1`))
  (`KismetArrayLibrary.Array_Add` _arr_spotlight (`self.SpotLight2`))
  (`KismetArrayLibrary.Array_Add` _arr_spotlight (`self.SpotLight3`))
  (`KismetArrayLibrary.Array_Add` _arr_spotlight (`self.SpotLight4`))
  (for _array_element_2 _arr_spotlight
    (`LightComponent.SetIntensity` _array_element_2 0.0)))

(event `Hoverd`
  (`MaterialInstanceDynamic.SetScalarParameterValue` (`|GetArrayItem` (`self.arr_Light`) (`self.Voted_Num`)) "LightPanner" 1.0)
  (`LightComponent.SetIntensity` (`|GetArrayItem` (`self.arr_SpotLight`) (`self.Voted_Num`)) 5000.0))

(event `Unhovered`
  (params (voted :type Integer))
  (`MaterialInstanceDynamic.SetScalarParameterValue` (`|GetArrayItem` (`self.arr_Light`) voted) "LightPanner" 0.0)
  (`LightComponent.SetIntensity` (`|GetArrayItem` (`self.arr_SpotLight`) voted) 0.0))

(event `Clicked`
  (set `self.IsClicked` true)
  (`MaterialInstanceDynamic.SetScalarParameterValue` (`|GetArrayItem` (`self.arr_Light`) (`self.Voted_Num`)) "LightPanner" 1.0)
  (`LightComponent.SetIntensity` (`|GetArrayItem` (`self.arr_SpotLight`) (`self.Voted_Num`)) 5000.0))

(event `Reset`
  (`MaterialInstanceDynamic.SetScalarParameterValue` (`|GetArrayItem` (`self.arr_Light`) (`self.Voted_Num`)) "LightPanner" 0.0)
  (`LightComponent.SetIntensity` (`|GetArrayItem` (`self.arr_SpotLight`) (`self.Voted_Num`)) 0.0))

(fn `UserConstructionScript`)