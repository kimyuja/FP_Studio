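; BP_Sea is the sea actor, which changes its height once it is flagged as clear.
; Tick watches the Bisclear flag and, through a DoOnce, fires the Clear event a single time.
; Clear plays a timeline that drives the actor's Z location while keeping X and Y.
; A delayed Clear followed by a Whale level sequence is left unconnected and never runs.
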(event `self.ReceiveBeginPlay`)

(event `self.ReceiveTick`
  (params (DeltaSeconds :type "Float (single-precision)"))
  (if (`self.bisclear`)
    (`/Engine/EditorBlueprintResources/StandardMacros.DoOnce` false
      (:`Completed`
        (`self.clear`)))))

(event `clear`
  (bind (_returnvalue_x _returnvalue_y) (`KismetMathLibrary.BreakVector` (`self.K2_GetActorLocation`)))
  (bind (_direction _newtrack_0) (`Timeline|Timeline`)
    (:`Update`
      (`self.K2_SetActorLocation` (`KismetMathLibrary.MakeVector` _returnvalue_x _returnvalue_y _newtrack_0)))))

(fn `UserConstructionScript`)