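; Spotlight display actor that animates three spotlights and flashes random animal characters.
; Shortly after BeginPlay, a Timeline drives the rotation of the three spotlights, one track per light on pitch or yaw.
; Tick accumulates time and calls ShowCharactor every two seconds, which randomly shows the Cow, Turtle, Rabbit or Frog component for one second before hiding it again.
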(event `self.ReceiveBeginPlay`
  (`KismetSystemLibrary.Delay` 0.5)
  (bind (_direction _newtrack_0 _newtrack_1 _newtrack_2) (`Timeline|Timeline`)
    (:`Update`
      (`SceneComponent.K2_SetRelativeRotation` (`self.SpotLight`) (`KismetMathLibrary.MakeRotator` 0.0 _newtrack_0) false false)
      (`SceneComponent.K2_SetRelativeRotation` (`self.SpotLight1`) (`KismetMathLibrary.MakeRotator` -90.0 -70.0 _newtrack_1) false false)
      (`SceneComponent.K2_SetRelativeRotation` (`self.SpotLight2`) (`KismetMathLibrary.MakeRotator` 90.0 -70.0 _newtrack_2) false false))))

(event `self.ReceiveTick`
  (params (DeltaSeconds :type "Float (single-precision)"))
  (set `self.CurrentTime` (+ DeltaSeconds (`self.CurrentTime`)))
  (if (>= (`self.CurrentTime`) 2.0)
    (`self.ShowCharactor`)
    (set `self.CurrentTime` 0.0)))

(event `ShowCharactor`
  (bind _cow (`self.Cow`))
  (bind _turtle (`self.Turtle`))
  (bind _rabbit (`self.Rabbit`))
  (bind _frog (`self.Frog`))
  (switch `int` (`KismetMathLibrary.RandomInteger` 4)
    (:`0`
      (`SceneComponent.SetVisibility` _cow true false)
      (`KismetSystemLibrary.Delay` 1.0)
      (`SceneComponent.SetVisibility` _cow false false))
    (:`1`
      (`SceneComponent.SetVisibility` _turtle true false)
      (`KismetSystemLibrary.Delay` 1.0)
      (`SceneComponent.SetVisibility` _turtle false false))
    (:`2`
      (`SceneComponent.SetVisibility` _rabbit true false)
      (`KismetSystemLibrary.Delay` 1.0)
      (`SceneComponent.SetVisibility` _rabbit false false))
    (:`3`
      (`SceneComponent.SetVisibility` _frog true false)
      (`KismetSystemLibrary.Delay` 1.0)
      (`SceneComponent.SetVisibility` _frog false false))))

(fn `NewFunction`)

(fn `UserConstructionScript`)