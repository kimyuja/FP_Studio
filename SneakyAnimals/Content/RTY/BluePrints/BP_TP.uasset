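; BP_TP is a placeable teleporter that sends any actor entering its box trigger to one of five fixed world locations.
; The construction script uses PlaceMode to choose the destination and set the TextRender label to its name: WitchHouse, Vault, Submarine, SuperMarket or Home.
; On box overlap, the other actor is moved straight to that location without a sweep or any filtering by actor type.
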(event `self.ReceiveBeginPlay`)

(event `self.Box.OnComponentBeginOverlap`
  (params (OverlappedComponent :type "PrimitiveComponent Object Reference") (OtherActor :type "Actor Object Reference") (OtherComp :type "PrimitiveComponent Object Reference") (OtherBodyIndex :type Integer) (bFromSweep :type Boolean) (SweepResult :type "HitResult Structure (by ref)"))
  (`self.K2_SetActorLocation` OtherActor (`self.Destination`) false false))

(fn `UserConstructionScript`
  (switch `int` (`self.PlaceMode`)
    (:`0`
      (`TextRenderComponent.K2_SetText` (`self.TextRender`) (`self.Witch House`))
      (set `self.Destination` (50000.0 -50000.0 0.0)))
    (:`1`
      (`TextRenderComponent.K2_SetText` (`self.TextRender`) (`self.Vault`))
      (set `self.Destination` (-50000.0 -50000.0 0.0)))
    (:`2`
      (`TextRenderComponent.K2_SetText` (`self.TextRender`) (`self.Submarine`))
      (set `self.Destination` (50000.0 50000.0 0.0)))
    (:`3`
      (`TextRenderComponent.K2_SetText` (`self.TextRender`) (`self.SuperMarket`))
      (set `self.Destination` (-50000.0 50000.0 0.0)))
    (:`4`
      (`TextRenderComponent.K2_SetText` (`self.TextRender`) (`self.Home`))
      (set `self.Destination` (0.0 0.0 0.0)))))