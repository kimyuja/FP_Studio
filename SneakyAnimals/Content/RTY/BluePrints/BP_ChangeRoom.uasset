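; BP_ChangeRoom is a trigger box that switches the local player into a character customization view through the lobby controller.
; On BeginPlay it finds CameraActors matching its Tag variable.
; When a locally controlled BP_TestPlayer enters, it saves the current view target, blends to the first tagged camera and calls ToggleCharacterCustomization on PC_Lobby.
; When that player leaves, it restores the saved view and toggles customization again.
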(event `self.ReceiveBeginPlay`
  (bind _outactors (`GameplayStatics.GetAllActorsOfClassWithTag` "/Script/Engine.CameraActor" (`self.Tag`)))
  (set `self.Room` _outactors))

(event `self.Box.OnComponentBeginOverlap`
  (params (OverlappedComponent :type "PrimitiveComponent Object Reference") (OtherActor :type "Actor Object Reference") (OtherComp :type "PrimitiveComponent Object Reference") (OtherBodyIndex :type Integer) (bFromSweep :type Boolean) (SweepResult :type "HitResult Structure (by ref)"))
  (bind _returnvalue (`GameplayStatics.GetPlayerController` 0))
  (bind _asbp_test_player (cast `/Game/KSW/BluePrints/BP_TestPlayer` OtherActor))
  (if (`Pawn.IsLocallyControlled` _asbp_test_player)
    (bind _output_get (set `self.As BP Test Player` _asbp_test_player))
    (bind _output_get_2 (set `self.NewVar` (`Controller.GetViewTarget` _returnvalue)))
    (`PlayerController.SetViewTargetWithBlend` _returnvalue (`|GetArrayItem` (`self.Room`)) 1.0 "VTBlend_Linear" 0.0 false)
    (bind _aspc_lobby (cast `PC_Lobby` _returnvalue))
    (bind _output_get_3 (set `self.As PC Lobby` _aspc_lobby))
    (`PC_Lobby.Toggle_CharacterCustomization` _output_get_3)))

(event `self.Box.OnComponentEndOverlap`
  (params (OverlappedComponent :type "PrimitiveComponent Object Reference") (OtherActor :type "Actor Object Reference") (OtherComp :type "PrimitiveComponent Object Reference") (OtherBodyIndex :type Integer))
  (bind _asbp_test_player (cast `/Game/KSW/BluePrints/BP_TestPlayer` OtherActor))
  (if (== (stale `self.Box.OnComponentBeginOverlap` _output_get) _asbp_test_player)
    (`PlayerController.SetViewTargetWithBlend` (`GameplayStatics.GetPlayerController` 0) (stale `self.Box.OnComponentBeginOverlap` _output_get_2) 0.0 "VTBlend_Linear" 0.0 false)
    (`PC_Lobby.Toggle_CharacterCustomization` (`self.As PC Lobby`))))

(fn `UserConstructionScript`)