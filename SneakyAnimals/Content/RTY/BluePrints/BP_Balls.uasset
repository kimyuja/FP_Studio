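; BP_Balls is an actor with five sphere components that play a bouncing "boing" sound when they hit something.
; Each sphere's hit event plays the same sound at that sphere's world location, scaled by a VolumeMultiplier variable.
; A random pitch multiplier on each play varies the sound between impacts.
; The hit logic is duplicated per sphere, and there is no cooldown or impact-strength check.
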(event `self.Sphere.OnComponentHit`
  (params (HitComponent :type "PrimitiveComponent Object Reference") (OtherActor :type "Actor Object Reference") (OtherComp :type "PrimitiveComponent Object Reference") (NormalImpulse :type "Vector Structure") (Hit :type "HitResult Structure (by ref)"))
  (`GameplayStatics.PlaySoundAtLocation` "/Game/RTY/Sound/Reaction/boing-2-44164.boing-2-44164" (`SceneComponent.K2_GetComponentLocation` (`self.Sphere`)) (struct) (`self.Volume Multiplier`) (`KismetMathLibrary.RandomFloatInRange` 0.5 1.5) 0.0 null null null null))

(event `self.Sphere1.OnComponentHit`
  (params (HitComponent :type "PrimitiveComponent Object Reference") (OtherActor :type "Actor Object Reference") (OtherComp :type "PrimitiveComponent Object Reference") (NormalImpulse :type "Vector Structure") (Hit :type "HitResult Structure (by ref)"))
  (`GameplayStatics.PlaySoundAtLocation` "/Game/RTY/Sound/Reaction/boing-2-44164.boing-2-44164" (`SceneComponent.K2_GetComponentLocation` (`self.Sphere1`)) (struct) (`self.Volume Multiplier`) (`KismetMathLibrary.RandomFloatInRange` 0.5 1.5) 0.0 null null null null))

(event `self.Sphere2.OnComponentHit`
  (params (HitComponent :type "PrimitiveComponent Object Reference") (OtherActor :type "Actor Object Reference") (OtherComp :type "PrimitiveComponent Object Reference") (NormalImpulse :type "Vector Structure") (Hit :type "HitResult Structure (by ref)"))
  (`GameplayStatics.PlaySoundAtLocation` "/Game/RTY/Sound/Reaction/boing-2-44164.boing-2-44164" (`SceneComponent.K2_GetComponentLocation` (`self.Sphere2`)) (struct) (`self.Volume Multiplier`) (`KismetMathLibrary.RandomFloatInRange` 0.5 1.5) 0.0 null null null null))

(event `self.Sphere3.OnComponentHit`
  (params (HitComponent :type "PrimitiveComponent Object Reference") (OtherActor :type "Actor Object Reference") (OtherComp :type "PrimitiveComponent Object Reference") (NormalImpulse :type "Vector Structure") (Hit :type "HitResult Structure (by ref)"))
  (`GameplayStatics.PlaySoundAtLocation` "/Game/RTY/Sound/Reaction/boing-2-44164.boing-2-44164" (`SceneComponent.K2_GetComponentLocation` (`self.Sphere3`)) (struct) (`self.Volume Multiplier`) (`KismetMathLibrary.RandomFloatInRange` 0.5 1.5) 0.0 null null null null))

(event `self.Sphere4.OnComponentHit`
  (params (HitComponent :type "PrimitiveComponent Object Reference") (OtherActor :type "Actor Object Reference") (OtherComp :type "PrimitiveComponent Object Reference") (NormalImpulse :type "Vector Structure") (Hit :type "HitResult Structure (by ref)"))
  (`GameplayStatics.PlaySoundAtLocation` "/Game/RTY/Sound/Reaction/boing-2-44164.boing-2-44164" (`SceneComponent.K2_GetComponentLocation` (`self.Sphere4`)) (struct) (`self.Volume Multiplier`) (`KismetMathLibrary.RandomFloatInRange` 0.5 1.5) 0.0 null null null null))

(fn `UserConstructionScript`)