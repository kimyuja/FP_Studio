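; BP_PC_Gameplay is a gameplay player controller Blueprint that hooks the player into multiplayer chat.
; Pressing Enter opens or closes chat through MultiplayerChatC.
; GetPlayerName returns the Username from the PS_Gameplay player state's user profile, while GetPlayerTeam returns an empty string.
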(event `Key|Enter`
  (params (Key :type "Key Structure"))
  (:`Pressed`
    (`/Game/MultiplayerChat/Main/MultiplayerChat_C.Open / Close Chat` (`self.MultiplayerChat_C`))))

(fn `GetPlayerName`
  (returns (Name :type String))
  (bind _asps_gameplay (cast `PS_Gameplay` (`self.PlayerState`)))
  (return (`KismetTextLibrary.Conv_TextToString` (`.Username` (break `Structure_UserProfile` (`PS_Base.Player_UserProfile` _asps_gameplay))))))

(fn `GetPlayerTeam`
  (returns (Team :type String))
  (return ""))

(fn `UserConstructionScript`)